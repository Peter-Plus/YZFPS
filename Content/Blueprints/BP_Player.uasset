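; BP_Player is the first-person shooter player character, handling movement, look, jump, crouch, firing and health.
; Enhanced Input actions drive the controls, with fire calling the held weapon and playing a rifle montage on FPSMesh.
; AddWeapon attaches a weapon to a mesh socket and tells BP_FPSGameMode to create an enemy.
; TakeDamage clamps health, then has the game mode show the blood screen or a defeat game-over.
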(event Custom|AddWeapon
  (params (Weapon :type BP%20Player%20Weapon%20Object%20Reference))
  ;[1 1 1] 持有武器，将武器附加到玩家骨骼的指定插槽上
  (bind _output_get (Variables|Default|SetWeapon Weapon))
  (Transformation|AttachComponentToComponent _output_get (Variables|Default|GetFPSMesh) "WeaponPoint" "SnapToTarget" "SnapToTarget" "SnapToTarget" true)
  (Default|CreateEnemy (Variables|Default|GetGameMode)))

(event Custom|TakeDamage
  (params (DamageValue :type Float%20%28double-precision%29))
  ;[1 1 1] 玩家受伤-先判断自身血量是否大于0
  (if (> (Variables|Default|GetHealth) 0.0)
    ;[1 1 1] 更新玩家血量，扣除damage value
    (bind _output_get (Variables|Default|SetHealth (Math|Float|Clamp(Float) (- (Variables|Default|GetHealth) DamageValue) 0.0 (Variables|Default|GetMaxHealth))))
    ;[1 1 1] 判断剩余生命值是否为0，为0结束面板，否则播放血屏
    (if (<= _output_get 0.0)
      (Class|FPSGameModeBase|ShowGameOver (Variables|Default|GetGameMode) (Utilities|Text|MakeLiteralText "Defeat"))
      (else
        (Class|FPSGameModeBase|PlayBloodScreen (Variables|Default|GetGameMode))))))

(event Input|EnhancedActionEvents|EnhancedInputActionIA_Move
  (params (ActionValue :type Vector%202D%20Structure) (ElapsedSeconds :type Float%20%28double-precision%29) (TriggeredSeconds :type Float%20%28double-precision%29) (InputAction :type Input%20Action%20Object%20Reference :default "/Game/Input/Actions/IA_Move.IA_Move"))
  (bind (_x _y) (Math|Vector2D|BreakVector2D ActionValue))
  ;[1 1 1] 处理WASD移动输入
  (Pawn|Input|AddMovementInput (Transformation|GetActorForwardVector) _x false)
  (Pawn|Input|AddMovementInput (Transformation|GetActorRightVector) _y false))

(event Input|EnhancedActionEvents|EnhancedInputActionIA_Look
  (params (ActionValue :type Vector%202D%20Structure) (ElapsedSeconds :type Float%20%28double-precision%29) (TriggeredSeconds :type Float%20%28double-precision%29) (InputAction :type Input%20Action%20Object%20Reference :default "/Game/Input/Actions/IA_Look.IA_Look"))
  (bind (_x _y) (Math|Vector2D|BreakVector2D ActionValue))
  ;[1 1 1] IA_Look
  (Pawn|Input|AddControllerYawInput (* _x 0.9))
  (Pawn|Input|AddControllerPitchInput (* _y -0.9)))

(event Input|EnhancedActionEvents|EnhancedInputActionIA_Jump
  (params (ActionValue :type Boolean) (ElapsedSeconds :type Float%20%28double-precision%29) (TriggeredSeconds :type Float%20%28double-precision%29) (InputAction :type Input%20Action%20Object%20Reference :default "/Game/Input/Actions/IA_Jump.IA_Jump"))
  ;[1 1 1] IA_Jump
  (:Started
    (Character|Jump))
  (:Completed
    (Character|StopJumping)))

(event Input|EnhancedActionEvents|EnhancedInputActionIA_Fire
  (params (ActionValue :type Boolean) (ElapsedSeconds :type Float%20%28double-precision%29) (TriggeredSeconds :type Float%20%28double-precision%29) (InputAction :type Input%20Action%20Object%20Reference :default "/Game/Input/Actions/IA_Fire.IA_Fire"))
  ;[1 1 1] IA_Fire
  (:Started
    (bind _weapon (Variables|Default|GetWeapon)
      (:then
        (Default|Fire _weapon)
        (Animation|Montage|PlayMontage (Variables|Default|GetFPSMesh) "/Game/GameAssets/Animations/FPP_Animations/FPP_RifleFire_Montage.FPP_RifleFire_Montage"))
      (:else))))

(event Input|EnhancedActionEvents|EnhancedInputActionIA_Crouch
  (params (ActionValue :type Boolean) (ElapsedSeconds :type Float%20%28double-precision%29) (TriggeredSeconds :type Float%20%28double-precision%29) (InputAction :type Input%20Action%20Object%20Reference :default "/Game/Input/Actions/IA_Crouch.IA_Crouch"))
  ;[1 1 1] IA_Crouch
  (:Started
    (Character|Crouch))
  (:Completed
    (Character|UnCrouch)))

(event EventBeginPlay
  ;[1 1 1] 绑定输入映射
  (Input|AddMappingContext (PlayerController|LocalPlayerSubsystems|GetEnhancedInputLocalPlayerSubsystem (Game|GetPlayerController 0)) "/Game/Input/IMC_DefaultContext.IMC_DefaultContext" 0 "(bIgnoreAllPressedKeysUntilRelease=True,bForceImmediately=False,bNotifyUserSettings=False)")
  (Variables|Default|SetMaxHealth (Variables|Default|GetHealth))
  (bind _asbp_fpsgame_mode (Utilities|Casting|CastToBP_FPSGameMode (Game|GetGameMode)))
  (Variables|Default|SetGameMode _asbp_fpsgame_mode))

(fn ConstructionScript)