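; BP_FPSGameMode is the FPS game mode Blueprint that owns the main HUD and relays game events to it.
; On game start it creates and displays UMG_Main and sets game-only input with a hidden cursor.
; Its events trigger the spawn-enemies hint, blood screen animation and game-over panel on that widget, with game over switching to UI-only input and showing the cursor.
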(event EventOnGameStart
  (bind _returnvalue (Game|GetPlayerController 0))
  ;[1 1 1] 事件 1：Event On Game Start
  (bind _returnvalue_2 (UserInterface|CreateWidget "/Game/Blueprints/UI/UMG_Main.UMG_Main_C"))
  (Variables|Default|SetMainUI _returnvalue_2)
  (UserInterface|Viewport|AddtoViewport _returnvalue_2 0)
  (Input|SetInputModeGameOnly _returnvalue false)
  (Variables|/Script/Engine.PlayerController|SetbShowMouseCursor _returnvalue false))

(event EventOnSpawnHint
  ;[1 1 1] 事件 2：Event On Spawn Hint
  (Development|PrintString "Hello")
  (Default|ShowSpawnEnemies (Variables|Default|GetMainUI)))

(event EventOnPlayBloodScreen
  ;[1 1 1] 事件 3：Event On Play Blood Screen
  (Default|PlayBloodScreenAnim (Variables|Default|GetMainUI)))

(event EventOnShowGameOver
  (params (Message :type Text%20%28by%20ref%29))
  (bind _returnvalue (Game|GetPlayerController 0))
  (Default|ShowGameOverPanel (Variables|Default|GetMainUI) Message)
  (Input|SetInputModeUIOnly _returnvalue 0 "DoNotLock" false)
  (Variables|/Script/Engine.PlayerController|SetbShowMouseCursor _returnvalue true))

(fn ConstructionScript)