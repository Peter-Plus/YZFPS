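; BP_Bullet is a projectile bullet that damages enemies and plays impact feedback on hit.
; SetVelocity aims the ProjectileMovement component at a target position at a fixed speed.
; On a sphere component hit it plays an impact sound, then casts the hit actor to BP_EnemyBase to deal damage with a body-hit effect, or spawns a metal impact effect otherwise, and destroys itself.
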(event OnComponentHit(Sphere)
  (params (HitComponent :type Primitive%20Component%20Object%20Reference) (OtherActor :type Actor%20Object%20Reference) (OtherComp :type Primitive%20Component%20Object%20Reference) (NormalImpulse :type Vector :default "0, 0, 0") (Hit :type Hit%20Result%20Structure%20%28by%20ref%29))
  (Audio|PlaySoundatLocation "/Game/GameAssets/WeaponEffects/Sound/Rifle/Rifle_ImpactSurface_Cue.Rifle_ImpactSurface_Cue" (Transformation|GetActorLocation) "0, 0, 0" 1.0 1.0 0.0 0 0 0 0)
  ;[1 1 1] 根据命中对象类型播放不同特效
  (bind _asbp_enemy_base (Utilities|Casting|CastToBP_EnemyBase OtherActor)
    (:then
      ;[1 1 1] 如果是敌人就播放飙血特效
      (Default|TakeDamage _asbp_enemy_base 2e+01)
      (Effects|SpawnEmitteratLocation "/Game/GameAssets/Effects/ParticleSystems/Gameplay/Player/P_body_bullet_impact.P_body_bullet_impact" (Transformation|GetActorLocation)))
    (:CastFailed
      (Effects|SpawnEmitteratLocation "/Game/GameAssets/WeaponEffects/FX/P_Impact_Metal_Medium_01.P_Impact_Metal_Medium_01" (Transformation|GetActorLocation))))
  (Actor|DestroyActor))

(event Custom|SetVelocity
  (params (TargetPos :type Vector))
  (Variables|/Script/Engine.MovementComponent|SetVelocity (Variables|Default|GetProjectileMovement) (* (Math|Vector|Normalize (- TargetPos (Transformation|GetActorLocation))) 5e+03)))

(event EventBeginPlay)

(event Collision|EventActorBeginOverlap
  (params (OtherActor :type Actor%20Object%20Reference)))

(event EventTick
  (params (DeltaSeconds :type Float%20%28single-precision%29)))

(fn ConstructionScript)