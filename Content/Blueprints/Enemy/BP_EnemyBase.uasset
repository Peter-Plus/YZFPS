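; Base enemy character for an FPS, driven by a behavior tree and showing a health bar widget.
; Sighting the player or taking damage sets the AttackTarget blackboard key.
; Attacks play a random montage whose notify sphere-traces forward to damage the player, then signal attack end.
; Hits play a reaction montage that halts movement, while death stops AI, removes health bar and collision, and notifies the game mode.
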(event OnSeePawn(PawnSensing)
  (params (Pawn :type Pawn%20Object%20Reference))
  (bind _asbp_player (Utilities|Casting|CastToBP_Player Pawn))
  (AI|Components|Blackboard|SetValueasObject (AI|GetBlackboard 0) (Utilities|Name|MakeLiteralName "AttackTarget") _asbp_player))

(event Custom|PlayAttack
  (bind _returnvalue (Transformation|GetActorLocation))
  ;[1 1 1] 播放攻击动画并调用攻击事件
  (bind _notifyname (Animation|Montage|PlayMontage (Variables|Character|GetMesh) (.OutItem (Utilities|Array|Random (Variables|Default|GetAttackMontageList))))
    (:OnCompleted
      _)
    (:OnInterrupted
      _)
    (:OnNotifyBegin
      (switch name _notifyname
        (:EAD
          (bind _outhits (Collision|MultiSphereTraceForObjects _returnvalue (+ _returnvalue (* (Transformation|GetActorForwardVector) 2e+02)) 5e+01 (Utilities|Array|MakeArray "ObjectTypeQuery3") false 0 "None"))
          (bind _array_element (Utilities|Array|ForEachLoopwithBreak _outhits :!label _label)
            (:LoopBody
              (bind _asbp_player (Utilities|Casting|CastToBP_Player (.HitActor (Collision|BreakHitResult _array_element))))
              (Default|TakeDamage _asbp_player (Math|Random|RandomFloatinRange 2e+01 3e+01))
              (goto _label Break)))))))
  (Default|CallEDAttackEnd))

(event Custom|TakeDamage
  (params (DamageValue :type Float%20%28double-precision%29))
  ;[1 1 1] 敌人生命大于0时扣血
  (if (> (Variables|Default|GetHealth) 0.0)
    (bind _output_get (Variables|Default|SetHealth (- (Variables|Default|GetHealth) DamageValue)))
    ;[1 1 1] 判断生命是否小于0
    (if (<= _output_get 0.0)
      (Variables|Default|SetIsDead true)
      (AI|Logic|StopLogic (Variables|/Script/AIModule.AIController|GetBrainComponent (Variables|Default|GetAIController)) "")
      (Components|DestroyComponent (Variables|Default|GetHealthBar))
      (Collision|SetCollisionEnabled (Variables|Character|GetMesh) "NoCollision")
      (Collision|SetCollisionEnabled (Variables|Default|GetCapsuleComponent) "NoCollision")
      (bind _asbp_fpsgame_mode (Utilities|Casting|CastToBP_FPSGameMode (Game|GetGameMode)))
      (Default|SetEnemyDie _asbp_fpsgame_mode self)
      (else
        (AI|Components|Blackboard|SetValueasObject (AI|GetBlackboard 0) (Utilities|Name|MakeLiteralName "AttackTarget") (Game|GetPlayerCharacter 0))
        ;[1 1 1] 播放伤害并限制移动
        (Animation|Montage|PlayMontage (Variables|Character|GetMesh) (Variables|Default|GetHitMontage)
          (:then
            (Pawn|Components|CharacterMovement|SetMovementMode (Variables|Character|GetCharacterMovement) "MOVE_None" 0 :!label _label))
          (:OnCompleted
            (Pawn|Components|CharacterMovement|SetMovementMode (Variables|Character|GetCharacterMovement) "MOVE_Walking" 0))
          (:OnInterrupted
            (goto _label)))))))

(event EventBeginPlay
  (bind _output_get (Variables|Default|SetAIController (AI|GetAIController self)))
  (AI|RunBehaviorTree _output_get "/Game/Blueprints/BT/BT_Enemy.BT_Enemy")
  (Variables|Default|SetMaxHealth (Variables|Default|GetHealth))
  (bind _returnvalue (UserInterface|CreateWidget "/Game/Blueprints/UI/UMG_EnemyHealth.UMG_EnemyHealth_C" 0 self))
  (UserInterface|SetWidget (Variables|Default|GetHealthBar) _returnvalue))

(fn ConstructionScript)