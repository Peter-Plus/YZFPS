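; BP_PlayerWeapon1 is a pickup weapon that spins in the world until the player overlaps its sphere and takes it.
; On overlap it disables collision, registers itself through BP_Player's AddWeapon, stops spinning and zeroes its rotation and mesh offset.
; Fire spawns a BP_Bullet at the ShootPoint socket and restarts audio and particle effects.
; It aims the bullet by tracing from screen center, passing the hit point or 200 m endpoint to SetVelocity.
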(event OnComponentBeginOverlap(Sphere)
  (params (OverlappedComponent :type Primitive%20Component%20Object%20Reference) (OtherActor :type Actor%20Object%20Reference) (OtherComp :type Primitive%20Component%20Object%20Reference) (OtherBodyIndex :type Integer) (bFromSweep :type Boolean) (SweepResult :type Hit%20Result%20Structure%20%28by%20ref%29))
  ;[1 1 1] 当玩家和武器发生碰撞的时候，将武器添加到玩家手上
  (bind _asbp_player (Utilities|Casting|CastToBP_Player OtherActor))
  (Collision|SetCollisionEnabled (Variables|Default|GetSphere) "NoCollision")
  (Default|AddWeapon _asbp_player self)
  ;[1 1 1] 停止旋转，设置武器的相对位置偏移为0
  (Variables|Default|SetIsEquip true)
  (Transformation|SetActorRelativeRotation "0, 0, 0")
  (Transformation|SetRelativeLocation (Variables|Default|GetWeaponMesh) "0, 0, 0" false false))

(event Custom|Fire
  (bind _returnvalue (Viewport|GetViewportSize))
  (bind _returnvalue_2 (Game|GetPlayerController 0))
  (bind _returnvalue_3 (/ _returnvalue 2.0))
  (bind (_worldposition _worlddirection) (Class|GameplayStatics|DeprojectScreentoWorld _returnvalue_2 _returnvalue_3))
  (bind _returnvalue_4 (* _worlddirection 2e+04))
  (bind _returnvalue_5 (+ _worldposition _returnvalue_4))
  (bind _returnvalue_6 (Game|SpawnActorfromClass "/Game/Blueprints/BP_Bullet.BP_Bullet_C" (Transformation|GetSocketTransform (Variables|Default|GetWeaponMesh) "ShootPoint" "RTS_World") "Undefined" "MultiplyWithRoot" 0 0))
  (Components|Activation|SetActive (Variables|Default|GetAudio) true true)
  (Components|Activation|SetActive (Variables|Default|GetParticleSystem) true true)
  (bind (_outhit _returnvalue_7) (Collision|LineTraceByChannel _worldposition _returnvalue_5 "TraceTypeQuery1" false 0 "None"))
  ;[1 1 1] 如果射线检测到碰撞获取碰撞点，否则获取200m的终点
  (Default|SetVelocity _returnvalue_6 (select _returnvalue_7 (.Location (Collision|BreakHitResult _outhit)) _returnvalue_5)))

(event EventBeginPlay
  (Components|Activation|SetActive (Variables|Default|GetAudio) false false)
  (Components|Activation|SetActive (Variables|Default|GetParticleSystem) false false))

(event EventTick
  (params (DeltaSeconds :type Float%20%28single-precision%29))
  (if (not (Variables|Default|GetIsEquip))
    (Class|Actor|AddActorWorldRotation "0.000000,3.000000,0.000000")))

(fn ConstructionScript)